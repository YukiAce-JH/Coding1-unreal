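; Falling platform actor that drops after the player character steps on its trigger box, then returns to its start for reuse.
; An overlap while ready runs chained activated, falling and resetting events separated by delays, with a ready flag blocking retriggers and material swaps showing each state.
; The fall uses physics simulation; resetting disables it and a timeline lerps the platform from its fallen transform back to the one saved at BeginPlay.
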(event `self.ReceiveBeginPlay`
  (set `self.originaltransform` (`SceneComponent.K2_GetComponentToWorld` (`self.platform`)))
  (`PrimitiveComponent.SetMaterial` (`self.platform`) 0 "/Game/materials/platformmt/M_readyPlat.M_readyPlat"))

(event `self.box trigger.OnComponentBeginOverlap`
  (params (OverlappedComponent :type "PrimitiveComponent Object Reference") (OtherActor :type "Actor Object Reference") (OtherComp :type "PrimitiveComponent Object Reference") (OtherBodyIndex :type Integer) (bFromSweep :type Boolean) (SweepResult :type "HitResult Structure (by ref)"))
  (`KismetSystemLibrary.PrintString` "something ran into  my trigger")
  (if (`self.IsReady`)
    (cast `/Game/Blueprints/BP_ThirdPersonCharacter` OtherActor)
    (`self.activated`)))

(event `activated`
  (`KismetSystemLibrary.PrintString` "activated")
  (`PrimitiveComponent.SetMaterial` (`self.platform`) 0 "/Game/materials/platformmt/M_Activatedplat.M_Activatedplat")
  (set `self.IsReady` false)
  (`KismetSystemLibrary.Delay` (`self.fall delay duration`))
  (`self.falling`))

(event `falling`
  (`KismetSystemLibrary.PrintString` "falling")
  (`PrimitiveComponent.SetMaterial` (`self.platform`) 0 "/Game/materials/platformmt/M_fallingplat.M_fallingplat")
  (`PrimitiveComponent.SetSimulatePhysics` (`self.platform`) true)
  (`KismetSystemLibrary.Delay` (`self.fall Duration`))
  (`self.resetting`))

(event `resetting`
  (`KismetSystemLibrary.PrintString` "resetting")
  (`PrimitiveComponent.SetMaterial` (`self.platform`) 0 "/Game/materials/platformmt/M_resetting.M_resetting")
  (set `self.fallentransform` (`SceneComponent.K2_GetComponentToWorld` (`self.platform`)))
  (`PrimitiveComponent.SetSimulatePhysics` (`self.platform`) false)
  (bind (_direction _newtrack_1) (`Timeline|returntostart` :!via `PlayFromStart`)
    (:`Update`
      (bind (_returnvalue_location _returnvalue_rotation) (`KismetMathLibrary.BreakTransform` (`KismetMathLibrary.TLerp` (`self.fallentransform`) (`self.originaltransform`) _newtrack_1)))
      (`SceneComponent.K2_SetWorldLocationAndRotation` (`self.platform`) _returnvalue_location _returnvalue_rotation false false))
    (:`Finished`
      (set `self.IsReady` true))))

(fn `UserConstructionScript`)