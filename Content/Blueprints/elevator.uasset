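; A falling platform actor, named elevator, that drops after the third-person character overlaps either of two trigger components, then returns to its starting pose.
; Activated, Falling and Resetting chain through delays, swapping the cube's material at each stage and using physics simulation for the drop.
; A timeline lerps the cube from its fallen transform back to the one cached at BeginPlay, then re-arms the triggers through the Start flag.
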(event `self.ReceiveBeginPlay`
  (set `self.transform` (`SceneComponent.K2_GetComponentToWorld` (`self.Cube`)))
  (`PrimitiveComponent.SetMaterial` (`self.Cube`) 0 "/Game/materials/platformmt/M_readyPlat.M_readyPlat"))

(event `self.point A.OnComponentBeginOverlap`
  (params (OverlappedComponent :type "PrimitiveComponent Object Reference") (OtherActor :type "Actor Object Reference") (OtherComp :type "PrimitiveComponent Object Reference") (OtherBodyIndex :type Integer) (bFromSweep :type Boolean) (SweepResult :type "HitResult Structure (by ref)"))
  (`KismetSystemLibrary.PrintString` "something ran into  my trigger")
  (if (`self.start`)
    (cast `/Game/Blueprints/BP_ThirdPersonCharacter` OtherActor)
    (`self.Activated`)))

(event `self.point b.OnComponentBeginOverlap`
  (params (OverlappedComponent :type "PrimitiveComponent Object Reference") (OtherActor :type "Actor Object Reference") (OtherComp :type "PrimitiveComponent Object Reference") (OtherBodyIndex :type Integer) (bFromSweep :type Boolean) (SweepResult :type "HitResult Structure (by ref)"))
  (`KismetSystemLibrary.PrintString` "something ran into  my trigger")
  (if (`self.start`)
    (cast `/Game/Blueprints/BP_ThirdPersonCharacter` OtherActor)
    (`self.Activated`)))

(event `Activated`
  (`KismetSystemLibrary.PrintString` "activated")
  (`PrimitiveComponent.SetMaterial` (`self.Cube`) 0 "/Game/materials/platformmt/M_Activatedplat.M_Activatedplat")
  (set `self.start` false)
  (`KismetSystemLibrary.Delay` 1.0)
  (`self.Falling`))

(event `Falling`
  (`KismetSystemLibrary.PrintString` "falling")
  (`PrimitiveComponent.SetMaterial` (`self.Cube`) 0 "/Game/materials/platformmt/M_fallingplat.M_fallingplat")
  (`PrimitiveComponent.SetSimulatePhysics` (`self.Cube`) true)
  (`KismetSystemLibrary.Delay` 3.0)
  (`self.Resetting`))

(event `Resetting`
  (`KismetSystemLibrary.PrintString` "resetting")
  (`PrimitiveComponent.SetMaterial` (`self.Cube`) 0 "/Game/materials/platformmt/M_resetting.M_resetting")
  (set `self.fallen transform` (`SceneComponent.K2_GetComponentToWorld` (`self.Cube`)))
  (`PrimitiveComponent.SetSimulatePhysics` (`self.Cube`) false)
  (bind (_direction _newtrack_1) (`Timeline|Timeline` :!via `PlayFromStart`)
    (:`Update`
      (bind (_returnvalue_location _returnvalue_rotation) (`KismetMathLibrary.BreakTransform` (`KismetMathLibrary.TLerp` (`self.fallen transform`) (`self.transform`) _newtrack_1)))
      (`SceneComponent.K2_SetWorldLocationAndRotation` (`self.Cube`) _returnvalue_location _returnvalue_rotation false false))
    (:`Finished`
      (set `self.start` true)
      (`PrimitiveComponent.SetMaterial` (`self.Cube`) 0 "/Game/materials/platformmt/M_readyPlat.M_readyPlat"))))

(fn `UserConstructionScript`)