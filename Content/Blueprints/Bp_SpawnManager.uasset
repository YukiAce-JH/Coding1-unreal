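; Spawn manager actor that populates the level with enemies and sends reinforcement waves.
; Shortly after BeginPlay it visits every Bp_SpawnPoint and, on a weighted random roll, usually spawns a Bp_Enemy at that point's transform.
; A wave check event, not called within this Blueprint, counts living enemy actors and re-runs the spawn after a delay when one or none remain.
; Progress is reported through debug prints.
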(event `self.ReceiveBeginPlay`
  (`KismetSystemLibrary.PrintString` "spawn manager exists")
  (`KismetSystemLibrary.Delay` 1.0)
  (`self.spawn enemies`))

(event `spawn enemies`
  (bind _outactors (`GameplayStatics.GetAllActorsOfClass` "/Game/Blueprints/Bp_SpawnPoint.Bp_SpawnPoint_C"))
  (for _array_element _outactors
    (`KismetSystemLibrary.PrintString` (`KismetSystemLibrary.GetDisplayName` _array_element) true true (struct :`R` 0.284729 :`G` 1.0 :`B` 0.740717 :`A` 1.0) 3.0)
    (if (`KismetMathLibrary.RandomBoolWithWeight` 0.8)
      (`|SpawnActorFromClass` "/Game/Blueprints/Bp_Enemy.Bp_Enemy_C" (`SceneComponent.K2_GetComponentToWorld` (`/Game/Blueprints/Bp_SpawnPoint.DefaultSceneRoot` _array_element)) "Undefined" "MultiplyWithRoot" null null)))
  (`KismetSystemLibrary.PrintString` "done!"))

(event `New wave check`
  (`KismetSystemLibrary.PrintString` "Time for reinforcements!")
  (bind _outactors (`GameplayStatics.GetAllActorsOfClass` "/Game/Blueprints/Bp_Enemy.Bp_Enemy_C"))
  (bind _returnvalue (`KismetArrayLibrary.Array_Length` _outactors))
  (`KismetSystemLibrary.PrintString` (`KismetStringLibrary.Concat_StrStr` "there are" (`KismetStringLibrary.Conv_IntToString` _returnvalue) "enemies in the level"))
  (if (> _returnvalue 1)
    (`KismetSystemLibrary.PrintString` "I STAND ALONE!")
    (else
      (`KismetSystemLibrary.PrintString` "THE CALVARY ARRIVES" true true (struct :`R` 1.0 :`G` 0.176752 :`B` 0.403126 :`A` 1.0))
      (`KismetSystemLibrary.Delay` 3.0)
      (`self.spawn enemies`))))

(fn `UserConstructionScript`)